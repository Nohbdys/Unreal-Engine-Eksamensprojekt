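; ArmorButton_BP is an armor upgrade button that sells the player armor levels at a price that rises with each level.
; SetUpgrade initializes the price once, calls Pay on the first FirstPersonCharacter found, then checks its CanAfford flag.
; On success it raises ArmorUpgLevel by a tenth, derives the next price linearly from it and increases Armor in proportion to it.
; It also refreshes a TextRenderActor showing price, current level and next level.
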(event `self.SetUpgrade`
  ;[1 1 1] Tilføjer et 0.1 til ArmorUpgLevel ( Svarer til 1 level )
  (`|ExecutionSequence`
    (:`then_0`
      (`/Engine/EditorBlueprintResources/StandardMacros.DoOnce` false
        (:`Completed`
          (set `self.Price` 150.0))))
    (:`then_1`
      (bind _outactors (`GameplayStatics.GetAllActorsOfClass` "/Game/FirstPersonCPP/Blueprints/FirstPersonCharacter.FirstPersonCharacter_C"))
      (bind _output (`|GetArrayItem` _outactors))
      (`/Game/FirstPersonCPP/Blueprints/FirstPersonCharacter.Pay` _output (`self.Price`))
      (if (`/Game/FirstPersonCPP/Blueprints/FirstPersonCharacter.CanAfford` _output)
        (`|ExecutionSequence`
          (:`then_0`
            (bind _outactors_2 (`GameplayStatics.GetAllActorsOfClass` "/Game/FirstPersonCPP/Blueprints/FirstPersonCharacter.FirstPersonCharacter_C"))
            (bind _output_2 (`|GetArrayItem` _outactors_2))
            (bind _output_get (set `/Game/FirstPersonCPP/Blueprints/FirstPersonCharacter.ArmorUpgLevel` (+ (`/Game/FirstPersonCPP/Blueprints/FirstPersonCharacter.ArmorUpgLevel` _output_2) 0.1) _output_2))
            (`|ExecutionSequence`
              (:`then_0`
                (bind _returnvalue (* (- _output_get 1.0) 10.0))
                ;[1 1 1] Sætter tallet på prisen
                (set `self.TmpString` (`KismetStringLibrary.Conv_IntToString` (`KismetMathLibrary.Round` _returnvalue)))
                (bind _returnvalue_2 (* _returnvalue 150.0))
                (set `self.Price` _returnvalue_2))
              (:`then_1`
                ;[1 1 1] Sætter teksten på Text Render
                (set `self.TextString` (`KismetStringLibrary.Concat_StrStr` "       Armor \nPrice: " (`KismetStringLibrary.Conv_IntToString` (`KismetMathLibrary.Round` _returnvalue_2)) "$ \nCurrent level: " (`KismetStringLibrary.Conv_IntToString` (`KismetMathLibrary.Round` (- _returnvalue 1.0))) " \nNext Level: " (`self.TmpString`)))
                (`TextRenderComponent.K2_SetText` (`TextRenderActor.TextRender` (`self.TextRenderActor`)) (`KismetTextLibrary.Conv_StringToText` (`self.TextString`))))))
          (:`then_1`
            (set `self.PlayerUpgString` (`self.TmpString`)))
          (:`then_2`
            ;;[1 1 1] Applies new armor upgrades
            (set `/Game/FirstPersonCPP/Blueprints/FirstPersonCharacter.Armor` (`KismetMathLibrary.Conv_IntToDouble` (`KismetMathLibrary.Round` (+ (`/Game/FirstPersonCPP/Blueprints/FirstPersonCharacter.Armor` _output_2) (* (`/Game/FirstPersonCPP/Blueprints/FirstPersonCharacter.ArmorUpgLevel` _output_2) 3.0)))) _output_2)))))))

(fn `UserConstructionScript`
  (`parent.UserConstructionScript`))