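; Upgrade button actor that sells Overall Resist levels to the first-person character when its SetUpgrade event is called.
; While the character's OverallRes is above 50, it charges the current price through Pay and checks CanAfford.
; A successful purchase raises OverallResUpgLevel, lowers OverallRes, scales the next price with the level and rewrites a linked TextRender sign.
; The first price is set through a DoOnce, and an older upgrade chain remains unconnected.
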(event `self.SetUpgrade`
  ;[1 1 1] Tilføjer et 0.1 til ArmorUpgLevel ( Svarer til 1 level )
  (`|ExecutionSequence`
    (:`then_0`
      (`/Engine/EditorBlueprintResources/StandardMacros.DoOnce` false
        (:`Completed`
          (set `self.Price` 35.0))))
    (:`then_1`
      (bind _outactors (`GameplayStatics.GetAllActorsOfClass` "/Game/FirstPersonCPP/Blueprints/FirstPersonCharacter.FirstPersonCharacter_C"))
      (bind _output (`|GetArrayItem` _outactors))
      (if (> (`/Game/FirstPersonCPP/Blueprints/FirstPersonCharacter.OverallRes` _output) 50.0)
        (`/Game/FirstPersonCPP/Blueprints/FirstPersonCharacter.Pay` _output (`self.Price`))
        (if (`/Game/FirstPersonCPP/Blueprints/FirstPersonCharacter.CanAfford` _output)
          (`|ExecutionSequence`
            (:`then_0`
              (bind _outactors_2 (`GameplayStatics.GetAllActorsOfClass` "/Game/FirstPersonCPP/Blueprints/FirstPersonCharacter.FirstPersonCharacter_C"))
              (bind _output_2 (`|GetArrayItem` _outactors_2))
              (bind _output_get (set `/Game/FirstPersonCPP/Blueprints/FirstPersonCharacter.OverallResUpgLevel` (+ (`/Game/FirstPersonCPP/Blueprints/FirstPersonCharacter.OverallResUpgLevel` _output_2) 0.1) _output_2))
              (`|ExecutionSequence`
                (:`then_0`
                  (bind _returnvalue (* (- _output_get 1.0) 10.0))
                  (bind _returnvalue_2 (`KismetMathLibrary.Round` _returnvalue))
                  ;[1 1 1] Skriver max i stedet for tal, hvis man er nået max lvl ( 12 )
                  (if (>= _returnvalue_2 26)
                    (set `self.TmpString` "Max")
                    (else
                      (set `self.TmpString` (`KismetStringLibrary.Conv_IntToString` _returnvalue_2))))
                  (bind _returnvalue_3 (* _returnvalue 350.0))
                  (set `self.Price` _returnvalue_3))
                (:`then_1`
                  ;[1 1 1] Sætter teksten på Text Render
                  (set `self.TextString` (`KismetStringLibrary.Concat_StrStr` "Overall Resist \nPrice: " (`KismetStringLibrary.Conv_IntToString` (`KismetMathLibrary.Round` _returnvalue_3)) "$ \nCurrent level: " (`KismetStringLibrary.Conv_IntToString` (`KismetMathLibrary.Round` (- _returnvalue 1.0))) " \nNext level: " (`self.TmpString`)))
                  (`TextRenderComponent.K2_SetText` (`TextRenderActor.TextRender` (`self.TextRenderActor`)) (`KismetTextLibrary.Conv_StringToText` (`self.TextString`))))))
            (:`then_1`
              (set `self.PlayerUpgString` (`self.TmpString`)))
            (:`then_2`
              ;;[1 1 1] Applies new armor upgrades
              (set `/Game/FirstPersonCPP/Blueprints/FirstPersonCharacter.OverallRes` (`KismetMathLibrary.Conv_IntToDouble` (`KismetMathLibrary.Round` (- (`/Game/FirstPersonCPP/Blueprints/FirstPersonCharacter.OverallRes` _output_2) 2.0))) _output_2))))))))

(fn `UserConstructionScript`
  (`parent.UserConstructionScript`))