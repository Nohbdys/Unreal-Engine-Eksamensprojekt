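; Pressable button actor intended for buying player upgrades, with an animated in-and-out press.
; A timeline, first played on BeginPlay, offsets the actor along X; finishing sets MoveInOut.
; ActivateButton uses that flag to block repeat presses, restarts the animation, calls SetUpgrade and prints debug text.
; SetUpgrade is empty: its switch raising FirstPersonCharacter upgrade levels when CanAfford is true is disconnected and never runs.
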(event `self.ReceiveBeginPlay`
  (bind (_direction _zposi) (`Timeline|Timeline_0`)
    (:`Update`
      (`self.K2_SetActorLocation` (+ (`KismetMathLibrary.MakeVector` _zposi) (`self.K2_GetActorLocation`))))
    (:`Finished`
      (set `self.MoveInOut` true))))

(fn `ActivateButton`
  ;[1 1 1] Tjekker om knappen er igang med at bevæge sig
  (if (`self.MoveInOut`)
    (`|ExecutionSequence`
      (:`then_0`
        ;[1 1 1] Starter animationen frem og tilbage for knappen
        (`TimelineComponent.PlayFromStart` (`self.Timeline_0`)))
      (:`then_1`
        ;[1 1 1] Sørger for man ikke kan trykke på knappen før den er færdig
        (set `self.MoveInOut` false))
      (:`then_2`
        (`self.SetUpgrade`))
      (:`then_3`
        (`KismetSystemLibrary.PrintString` (`self.PlayerUpgString`))
        (`KismetSystemLibrary.PrintString` "YOU PRESSED THE BUTTON")))))

(fn `SetUpgrade`)

(fn `UserConstructionScript`)