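; SmallRoom_BP is a transition room that sends the player into a random level when they enter its trigger.
; The overlap teleports the player by their room-relative offset with adjusted yaw, seemingly into a matching static start room.
; MapDataAndActions_BP then picks the level and spawns enemies, and the end door's height follows whether it is the shop.
; In parallel, StaticSmallRoom_BP1's door is reset and opened; a door timeline here is unused.
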(event `self.ReceiveTick`
  (params (DeltaSeconds :type "Float (single-precision)"))
  (bind _childactor (`ChildActorComponent.ChildActor` (`self.EndDoor_BP`)))
  (bind (_returnvalue_x _returnvalue_y) (`KismetMathLibrary.BreakVector` (`self.K2_GetActorLocation` _childactor)))
  (set `self.DeltaTime` DeltaSeconds)
  (`/Engine/EditorBlueprintResources/StandardMacros.DoOnce` false
    (:`Completed`
      (bind _outactors (`GameplayStatics.GetAllActorsOfClass` "/Game/FirstPersonCPP/Blueprints/FirstPersonCharacter.FirstPersonCharacter_C"))
      (set `self.PlayerRef` (`|GetArrayItem` _outactors))
      (bind _outactors_2 (`GameplayStatics.GetAllActorsOfClass` "/Game/OurContent/MapDataAndActions_BP.MapDataAndActions_BP_C"))
      (set `self.MapDataRef` (`|GetArrayItem` _outactors_2))
      (`self.K2_SetActorLocation` _childactor (`KismetMathLibrary.MakeVector` _returnvalue_x _returnvalue_y -1991.0) false false))))

(event `self.RandomTrigger.OnComponentBeginOverlap`
  (params (OverlappedComponent :type "PrimitiveComponent Object Reference") (OtherActor :type "Actor Object Reference") (OtherComp :type "PrimitiveComponent Object Reference") (OtherBodyIndex :type Integer) (bFromSweep :type Boolean) (SweepResult :type "HitResult Structure (by ref)"))
  (bind (_returnvalue_roll _returnvalue_pitch _returnvalue_yaw) (`KismetMathLibrary.BreakRotator` (`self.K2_GetActorRotation`)))
  (bind _mapdataref (`self.MapDataRef`))
  (bind _childactor (`ChildActorComponent.ChildActor` (`self.EndDoor_BP`)))
  (bind _childactor_2 (`ChildActorComponent.ChildActor` (`self.EndDoor_BP`)))
  (bind (_returnvalue_x _returnvalue_y) (`KismetMathLibrary.BreakVector` (`self.K2_GetActorLocation` _childactor)))
  (bind (_returnvalue_x_2 _returnvalue_y_2) (`KismetMathLibrary.BreakVector` (`self.K2_GetActorLocation` _childactor_2)))
  (if (== OtherActor (`GameplayStatics.GetPlayerPawn` 0))
    (`|ExecutionSequence`
      (:`then_0`
        (`self.K2_SetActorLocationAndRotation` (`self.PlayerRef`) (+ (* (- (`self.K2_GetActorLocation`) (`SceneComponent.K2_GetComponentLocation` (`Actor.RootComponent` (`self.PlayerRef`)))) -1.0) (0.0 0.0 -30.0)) (`KismetMathLibrary.MakeRotator` 0.0 0.0 (+ _returnvalue_yaw -90.0)) false true)
        ;[1 1 1] Skifter til en tilfældig bane
        (bind _outactors (`GameplayStatics.GetAllActorsOfClass` "/Game/OurContent/MapDataAndActions_BP.MapDataAndActions_BP_C"))
        (bind _output (`|GetArrayItem` _outactors))
        (`/Game/OurContent/MapDataAndActions_BP.RandomLevel` _output)
        (`KismetSystemLibrary.Delay` 0.2)
        ;[1 1 1] Spawner fjender
        (bind _amountspawned (`/Game/OurContent/MapDataAndActions_BP.SpawnEnemy` _output 27.0))
        (`KismetSystemLibrary.PrintString` (`KismetStringLibrary.Conv_DoubleToString` _amountspawned))
        ;[1 1 1] Rykker døren alt efter om man er i shoppen eller i et level
        (if (!= (`/Game/OurContent/MapDataAndActions_BP.CurrentLevel` _mapdataref) (`|GetArrayItem` (`/Game/OurContent/MapDataAndActions_BP.LevelArray` _mapdataref) 4))
          (`self.K2_SetActorLocation` _childactor (`KismetMathLibrary.MakeVector` _returnvalue_x _returnvalue_y 39.0) false false)
          (else
            (`self.K2_SetActorLocation` _childactor_2 (`KismetMathLibrary.MakeVector` _returnvalue_x_2 _returnvalue_y_2 -270.0) false false))))
      (:`then_1`
        ;[1 1 1] Åben og lukke døren i start lokalet
        (bind _outactors_2 (`GameplayStatics.GetAllActorsOfClass` "/Game/OurContent/Baner/StaticSmallRoom_BP1.StaticSmallRoom_BP1_C"))
        (bind _output_2 (`|GetArrayItem` _outactors_2))
        (bind _staticdoorref (`/Game/OurContent/Baner/StaticSmallRoom_BP1.StaticDoorRef` _output_2))
        (`self.K2_SetActorRotation` _staticdoorref (struct :`Yaw` 90.0) false)
        (bind (_returnvalue_x_3 _returnvalue_y_3) (`KismetMathLibrary.BreakVector` (`self.K2_GetActorLocation` _staticdoorref)))
        ;;[1 1 1] Lukker døren i start lokalet
        (`self.K2_SetActorLocation` _staticdoorref (`KismetMathLibrary.MakeVector` _returnvalue_x_3 _returnvalue_y_3 30.0) false true)
        ;;[1 1 1] Åbner døren i start lokalet
        (`/Game/OurContent/Baner/StaticSmallRoom_BP1.OpenDoor` _output_2 _staticdoorref)))))

(event `self.ReceiveBeginPlay`
  (set `self.EndPoint` (500.0 -500.0 0.0))
  (set `self.MapRotation` (`self.K2_GetActorRotation`)))

(fn `UserConstructionScript`)