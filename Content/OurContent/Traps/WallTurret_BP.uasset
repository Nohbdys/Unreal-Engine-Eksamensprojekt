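; WallTurret_BP is a wall turret trap that repeatedly fires BasicTrapBullet_BP projectiles from just ahead of itself along its forward vector.
; BeginPlay starts an endless loop with a random delay, shortened as Difficulty on MapDataAndActions_BP_Oliver rises, with a short random fallback.
; FireTurret spawns the bullet and switches on the light and steam effect, then is called again immediately to switch both off.
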(event `self.ReceiveBeginPlay`
  (bind _outactors (`GameplayStatics.GetAllActorsOfClass` "/Game/OurContent/MapDataAndActions_BP_Oliver.MapDataAndActions_BP_Oliver_C"))
  (bind _returnvalue (+ (`KismetMathLibrary.RandomFloatInRange` 2.0 5.0) (/ (* (- (`/Game/OurContent/MapDataAndActions_BP_Oliver.Difficulty` (`|GetArrayItem` _outactors)) 1.0) -1.0) 2.0)))
  (if (> _returnvalue 0.0) :!label _label
    (set `self.Delay` _returnvalue)
    (else
      (set `self.Delay` (`KismetMathLibrary.RandomFloatInRange` 0.5 1.0))))
  (`KismetSystemLibrary.Delay` (`self.Delay`))
  (`self.FireTurret` true)
  (`self.FireTurret` false)
  (goto _label))

(fn `FireTurret`
  (params (Fired :type Boolean))
  (bind _returnvalue (`ActorComponent.GetOwner` (`self.StaticMeshComponent`)))
  (if Fired
    (`LightComponent.SetIntensity` (`self.PointLight`) 10000.0)
    (`ActorComponent.Activate` (`self.P_Steam_Lit_2`) true)
    (`|SpawnActorFromClass` "/Game/OurContent/Traps/TrapBulletTypes/BasicTrapBullet_BP.BasicTrapBullet_BP_C" (`KismetMathLibrary.MakeTransform` (+ (`self.K2_GetActorLocation` _returnvalue) (* (`self.GetActorForwardVector` _returnvalue) 30.0)) (`self.K2_GetActorRotation` _returnvalue)) "AlwaysSpawn" "OverrideRootScale" null null)
    (else
      (`ActorComponent.Deactivate` (`self.P_Steam_Lit_2`))
      (`LightComponent.SetIntensity` (`self.PointLight`) 0.0))))

(fn `UserConstructionScript`)