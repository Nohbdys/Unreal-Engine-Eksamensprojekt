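; Spike trap actor that moves vertically and damages and snags the first-person player on contact.
; A looping timeline adds frame-time-scaled Z offsets to the actor's location, snapping back to the start position after each run to correct drift.
; Player overlap deals damage scaled by TrapRes, then a Gate loop repeatedly near-zeroes velocity with LaunchCharacter and reapplies damage.
; End overlap closes the gate and resets the entry hit.
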(event `self.ReceiveTick`
  (params (DeltaSeconds :type "Float (single-precision)"))
  (set `self.DeltaTime` DeltaSeconds))

(event `self.ReceiveBeginPlay`
  (`|ExecutionSequence`
    (:`then_0`
      ;[1 1 1] Sætter PlayerRef til FirstPersonCharacter, for nemmere at kunne tilgå den
      (bind _outactors (`GameplayStatics.GetAllActorsOfClass` "/Game/FirstPersonCPP/Blueprints/FirstPersonCharacter.FirstPersonCharacter_C"))
      (set `self.PlayerRef` (`|GetArrayItem` _outactors)))
    (:`then_1`
      ;[1 1 1] Gemmer start lokation, for at kunne resette dens position.
      (set `self.InitLocation` (`self.K2_GetActorLocation` (`ActorComponent.GetOwner` (`self.DefaultSceneRoot`)))))
    (:`then_2`
      ;[1 1 1] Bevæger spikes frem og tilbage, baseret på timeline værdier, og resetter dens position efter hver gennemkørelse, da timeline er lidt ustabil
      (bind (_direction _zposi) (`Timeline|SpikePosition` :!via `PlayFromStart` :!label _label)
        (:`Update`
          (`self.K2_SetActorLocation` (+ (`KismetMathLibrary.MakeVector` 0.0 0.0 (* _zposi (* (`self.DeltaTime`) 70.0))) (`self.K2_GetActorLocation` (`ActorComponent.GetOwner` (`self.DefaultSceneRoot`))))))
        (:`Finished`
          (`self.K2_SetActorLocation` (`self.InitLocation`))
          (switch `ETimelineDirection` _direction
            (:`Forward`
              (goto _label :!via `PlayFromStart`))
            (:`Backward`
              (goto _label :!via `ReverseFromEnd`))))))
    (:`then_3`
      (set `self.Damage` 20.0))))

(event `self.OverlapTrigger.OnComponentBeginOverlap`
  (params (OverlappedComponent :type "PrimitiveComponent Object Reference") (OtherActor :type "Actor Object Reference") (OtherComp :type "PrimitiveComponent Object Reference") (OtherBodyIndex :type Integer) (bFromSweep :type Boolean) (SweepResult :type "HitResult Structure (by ref)"))
  ;[1 1 1] Spike trap collision handle
  (if (== OtherActor (`self.PlayerRef`))
    (`|ExecutionSequence`
      (:`then_0`
        (`/Engine/EditorBlueprintResources/StandardMacros.DoOnce` false
          (:`Completed`
            (bind _outactors (`GameplayStatics.GetAllActorsOfClass` "/Game/FirstPersonCPP/Blueprints/FirstPersonCharacter.FirstPersonCharacter_C")))))
      (:`then_1`
        (`/Engine/EditorBlueprintResources/StandardMacros.DoOnce` false :!label _label_2
          (:`Completed`
            (bind _output (`|GetArrayItem` _outactors))
            (`/Game/FirstPersonCPP/Blueprints/FirstPersonCharacter.TakeDamage` _output (* (`self.Damage`) (/ (`/Game/FirstPersonCPP/Blueprints/FirstPersonCharacter.TrapRes` _output) 100.0)))
            (`KismetSystemLibrary.PrintString` "Player took dmg from trap"))))
      (:`then_2`
        (goto _label_3 :!via `Open`))
      (:`then_3`
        ;;[1 1 1] Sætter spilleren halvt fast, når dn træder i spikes, ved at sætte dens velocity til 0.
        (`/Engine/EditorBlueprintResources/StandardMacros.Gate` true :!label _label_3
          (:`Exit`
            (`Character.LaunchCharacter` (`self.PlayerRef`) (0.1 0.1 0.0) true true)
            (`KismetSystemLibrary.Delay` 0.1)
            (`Character.LaunchCharacter` (`self.PlayerRef`) (0.1 0.1 0.1) true true)
            (`KismetSystemLibrary.Delay` 0.1)
            (`Character.LaunchCharacter` (`self.PlayerRef`) (0.1 0.1 0.1) true true)
            (`KismetSystemLibrary.Delay` 0.1)
            (`Character.LaunchCharacter` (`self.PlayerRef`) (0.1 0.1 0.1) true true)
            (`KismetSystemLibrary.Delay` 0.1)
            (`/Game/FirstPersonCPP/Blueprints/FirstPersonCharacter.TakeDamage` _output (* (`self.Damage`) (/ (`/Game/FirstPersonCPP/Blueprints/FirstPersonCharacter.TrapRes` _output) 100.0)))
            (`KismetSystemLibrary.PrintString` "Player took dmg from trap")
            (goto _label_3)))))))

(event `self.OverlapTrigger.OnComponentEndOverlap`
  (params (OverlappedComponent :type "PrimitiveComponent Object Reference") (OtherActor :type "Actor Object Reference") (OtherComp :type "PrimitiveComponent Object Reference") (OtherBodyIndex :type Integer))
  ;[1 1 1] Spike trap collision handle
  (`|ExecutionSequence`
    (:`then_0`
      (goto _label_2 :!via `Reset`))
    (:`then_1`
      (goto _label_3 :!via `Close`))))

(fn `UserConstructionScript`)