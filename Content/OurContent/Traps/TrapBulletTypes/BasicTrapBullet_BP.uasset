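; BasicTrapBullet_BP is a trap projectile that damages the player and destroys itself on hitting the player or a MapDummy actor.
; Tick moves it a fixed step along the HitBox forward vector without sweep or delta-time scaling, so speed depends on frame rate.
; HitBox overlap with the player deals base damage multiplied by the character's TrapRes percentage.
; BeginPlay caches all MapDummy actors, but the array is unused here.
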(event `self.ReceiveBeginPlay`
  (set `self.Damage` 10.0)
  (bind _outactors (`GameplayStatics.GetAllActorsOfClass` "/Game/OurContent/MapDummy.MapDummy_C"))
  (set `self.Maps` _outactors))

(event `self.ReceiveTick`
  (params (DeltaSeconds :type "Float (single-precision)"))
  (`self.K2_SetActorLocation` (`ActorComponent.GetOwner` (`self.DefaultSceneRoot`)) (+ (* (`SceneComponent.GetForwardVector` (`self.HitBox`)) 8.0) (`self.K2_GetActorLocation`)) false false))

(event `self.HitBox.OnComponentBeginOverlap`
  (params (OverlappedComponent :type "PrimitiveComponent Object Reference") (OtherActor :type "Actor Object Reference") (OtherComp :type "PrimitiveComponent Object Reference") (OtherBodyIndex :type Integer) (bFromSweep :type Boolean) (SweepResult :type "HitResult Structure (by ref)"))
  (if (== OtherActor (`GameplayStatics.GetPlayerCharacter` 0))
    (bind _asfirst_person_character (cast `/Game/FirstPersonCPP/Blueprints/FirstPersonCharacter` OtherActor))
    (`/Game/FirstPersonCPP/Blueprints/FirstPersonCharacter.TakeDamage` _asfirst_person_character (* (`self.Damage`) (/ (`/Game/FirstPersonCPP/Blueprints/FirstPersonCharacter.TrapRes` _asfirst_person_character) 100.0)))
    (`self.K2_DestroyActor` (`ActorComponent.GetOwner` (`self.DefaultSceneRoot`)))
    (`KismetSystemLibrary.PrintString` "Destroyed by player")
    (else
      (cast `/Game/OurContent/MapDummy` OtherActor)
      (`self.K2_DestroyActor` (`ActorComponent.GetOwner` (`self.DefaultSceneRoot`))))))

(fn `UserConstructionScript`)