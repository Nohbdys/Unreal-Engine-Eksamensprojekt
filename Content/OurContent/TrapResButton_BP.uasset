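; TrapResButton_BP is an upgrade button that raises the player's TrapRes upgrade level, presumably trap resistance.
; When CanAfford is true, SetUpgrade adds one 0.1 step to TrapResUpgLevel on the first FirstPersonCharacter found.
; It then converts the multiplier into a whole level number and stores it as text in PlayerUpgString.
; The node comment mentions ArmorUpgLevel, but the code changes TrapResUpgLevel.
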(event `self.SetUpgrade`
  ;[1 1 1] Tilføjer et 0.1 til ArmorUpgLevel ( Svarer til 1 level )
  (if (`self.CanAfford`)
    (`|ExecutionSequence`
      (:`then_0`
        (bind _outactors (`GameplayStatics.GetAllActorsOfClass` "/Game/FirstPersonCPP/Blueprints/FirstPersonCharacter.FirstPersonCharacter_C"))
        (bind _output (`|GetArrayItem` _outactors))
        (bind _output_get (set `/Game/FirstPersonCPP/Blueprints/FirstPersonCharacter.TrapResUpgLevel` (+ (`/Game/FirstPersonCPP/Blueprints/FirstPersonCharacter.TrapResUpgLevel` _output) 0.1) _output))
        (set `self.TmpString` (`KismetStringLibrary.Conv_IntToString` (`KismetStringLibrary.Conv_StringToInt` (`KismetStringLibrary.Conv_DoubleToString` (* (- _output_get 1.0) 10.0))))))
      (:`then_1`
        (set `self.PlayerUpgString` (`self.TmpString`))))))

(fn `UserConstructionScript`
  (`parent.UserConstructionScript`))