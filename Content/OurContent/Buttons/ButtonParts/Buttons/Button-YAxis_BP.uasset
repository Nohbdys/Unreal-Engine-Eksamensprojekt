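; Pressable button actor that animates along the world Y axis and calls an upgrade hook when activated.
; A timeline, also played on BeginPlay, offsets the location each update, then snaps back to the start position to cancel drift.
; ActivateButton locks input until the animation finishes, calls the empty SetUpgrade and prints debug text.
; PlayBuzzer and PlayButton both spawn the same wrong-buzzer sound at a given location.
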(event `self.ReceiveBeginPlay`
  (set `self.StartPos` (`self.K2_GetActorLocation`))
  (bind (_direction _zposi) (`Timeline|Timeline_0`)
    (:`Update`
      (`self.K2_SetActorLocation` (- (`self.K2_GetActorLocation`) (`KismetMathLibrary.MakeVector` 0.0 _zposi))))
    (:`Finished`
      ;[1 1 1] Sørger for at knappen ikke rykker sig væk fra sit start punkt (Timeline driller)
      (set `self.MoveInOut` true)
      (`self.K2_SetActorLocation` (`self.StartPos`)))))

(fn `ActivateButton`
  ;[1 1 1] Tjekker om knappen er igang med at bevæge sig
  (if (`self.MoveInOut`)
    (`|ExecutionSequence`
      (:`then_0`
        ;[1 1 1] Starter animationen frem og tilbage for knappen
        (`TimelineComponent.PlayFromStart` (`self.Timeline_0`)))
      (:`then_1`
        ;[1 1 1] Sørger for man ikke kan trykke på knappen før den er færdig
        (set `self.MoveInOut` false))
      (:`then_2`
        (`self.SetUpgrade`))
      (:`then_3`
        (`KismetSystemLibrary.PrintString` (`self.PlayerUpgString`))
        (`KismetSystemLibrary.PrintString` "YOU PRESSED THE BUTTON")))))

(fn `PlayButton`
  (params (LocationToPlay :type "Vector Structure"))
  (`GameplayStatics.SpawnSoundAtLocation` "/Game/OurContent/Souund/Wrong_Buzzer.Wrong_Buzzer" LocationToPlay (struct) 1.0 1.0 0.0 "/Game/OurContent/Souund/Attenuations/Button_atten.Button_atten"))

(fn `PlayBuzzer`
  (params (LocationToPlay :type "Vector Structure"))
  (`GameplayStatics.SpawnSoundAtLocation` "/Game/OurContent/Souund/Wrong_Buzzer.Wrong_Buzzer" LocationToPlay (struct) 1.0 1.0 0.0 "/Game/OurContent/Souund/Attenuations/Button_atten.Button_atten"))

(fn `SetUpgrade`)

(fn `UserConstructionScript`)