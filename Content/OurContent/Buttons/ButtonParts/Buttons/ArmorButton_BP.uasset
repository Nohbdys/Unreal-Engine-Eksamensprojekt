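; Upgrade button that sells armor to the FirstPersonCharacter through its SetUpgrade event.
; While Armor is below HealthMax, it charges Price and, if affordable, raises ArmorUpgLevel, adds level-scaled armor, recalculates the price and plays a sound.
; It then writes price, levels and bonus to a TextRenderActor found once by searching object names for "Armor".
; At the armor cap it plays a buzzer instead.
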(event `self.SetUpgrade`
  ;[1 1 1] Opgraderer Armor (Tilføjer armor til spilleren)
  (`|ExecutionSequence`
    (:`then_0`
      (`/Engine/EditorBlueprintResources/StandardMacros.DoOnce` false
        (:`Completed`
          (set `self.Price` 75.0))))
    (:`then_1`
      (bind _outactors (`GameplayStatics.GetAllActorsOfClass` "/Game/FirstPersonCPP/Blueprints/FirstPersonCharacter.FirstPersonCharacter_C"))
      (bind _output (`|GetArrayItem` _outactors))
      (if (< (`/Game/FirstPersonCPP/Blueprints/FirstPersonCharacter.Armor` _output) (`/Game/FirstPersonCPP/Blueprints/FirstPersonCharacter.HealthMax` _output))
        (`/Game/FirstPersonCPP/Blueprints/FirstPersonCharacter.Pay` _output (`self.Price`))
        (if (`/Game/FirstPersonCPP/Blueprints/FirstPersonCharacter.CanAfford` _output)
          (`|ExecutionSequence`
            (:`then_0`
              (bind _outactors_2 (`GameplayStatics.GetAllActorsOfClass` "/Game/FirstPersonCPP/Blueprints/FirstPersonCharacter.FirstPersonCharacter_C"))
              (bind _output_2 (`|GetArrayItem` _outactors_2))
              (bind _output_get (set `/Game/FirstPersonCPP/Blueprints/FirstPersonCharacter.ArmorUpgLevel` (+ (`/Game/FirstPersonCPP/Blueprints/FirstPersonCharacter.ArmorUpgLevel` _output_2) 0.1) _output_2))
              (`|ExecutionSequence`
                (:`then_0`
                  (bind _returnvalue (* (- _output_get 1.0) 10.0))
                  ;[1 1 1] Sætter tallet på prisen
                  (set `self.TmpString` (`KismetStringLibrary.Conv_IntToString` (`KismetMathLibrary.Round` _returnvalue)))
                  (`|ExecutionSequence`
                    (:`then_0`
                      (`GameplayStatics.PlaySoundAtLocation` "/Game/OurContent/Souund/Thuum.Thuum" (`self.K2_GetActorLocation` (`ActorComponent.GetOwner` (`self.StaticMeshComponent`))) (struct) 1.0 1.0 0.0 "/Game/OurContent/Souund/Attenuations/Button_atten.Button_atten"))
                    (:`then_1`
                      (bind _returnvalue_2 (* _returnvalue 75.0))
                      (set `self.Price` _returnvalue_2))))
                (:`then_1`
                  ;[1 1 1] Tilføjer Nye armor opgraderinger
                  (bind _output_get_2 (set `/Game/FirstPersonCPP/Blueprints/FirstPersonCharacter.Armor` (`KismetMathLibrary.Conv_IntToDouble` (`KismetMathLibrary.Round` (+ (`/Game/FirstPersonCPP/Blueprints/FirstPersonCharacter.Armor` _output_2) (* (`/Game/FirstPersonCPP/Blueprints/FirstPersonCharacter.ArmorUpgLevel` _output_2) 3.0)))) _output_2)))
                (:`then_2`
                  ;[1 1 1] Ændrer teksten på TextRender
                  ;;[1 1 1] Sequence.
                  ;; 1: Finder den rigtige TextRender
                  ;; 2: Sætter teksten på TextRender
                  (set `self.TextString` (`KismetStringLibrary.Concat_StrStr` "       Armor \nPrice: " (`KismetStringLibrary.Conv_IntToString` (`KismetMathLibrary.Round` _returnvalue_2)) "$ \nCurrent level: " (`KismetStringLibrary.Conv_IntToString` (`KismetMathLibrary.Round` (- _returnvalue 1.0))) " \nNext level: " (`self.TmpString`) " \nCurrent bonus: \n+" (`KismetStringLibrary.Conv_DoubleToString` _output_get_2)))
                  (`|ExecutionSequence`
                    (:`then_0`
                      ;;[1 1 1] Finder TextRenderComponent, som har et navn der indeholder Armor og sætter den lig med TextRender
                      (`/Engine/EditorBlueprintResources/StandardMacros.DoOnce` false
                        (:`Completed`
                          (bind _outactors_3 (`GameplayStatics.GetAllActorsOfClass` "/Script/Engine.TextRenderActor"))
                          (for _array_element _outactors_3
                            (if (`KismetStringLibrary.Contains` (`KismetSystemLibrary.GetObjectName` _array_element) "Armor")
                              (set `self.TextRenderComponent` (`TextRenderActor.TextRender` _array_element))
                              (`KismetSystemLibrary.PrintString` "Found TextRender"))))))
                    (:`then_1`
                      (`TextRenderComponent.K2_SetText` (`self.TextRenderComponent`) (`KismetTextLibrary.Conv_StringToText` (`self.TextString`))))))))
            (:`then_1`
              (set `self.PlayerUpgString` (`self.TmpString`)))))
        (else
          (`self.PlayBuzzer` (`self.K2_GetActorLocation`)))))))

(fn `UserConstructionScript`
  (`parent.UserConstructionScript`))