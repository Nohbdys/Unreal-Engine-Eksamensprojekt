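; Speed upgrade button that sells the first-person character permanent walk-speed increases.
; SetUpgrade buzzes past the speed cap; otherwise it calls Pay and, if affordable, raises SpeedUpgLevel, compounds Speed and updates MaxWalkSpeed.
; Price scales linearly with level, with separate sounds for a normal or maxed upgrade.
; A TextRenderActor, found once by "Speed" in its name, shows price, levels and bonus percentage.
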(event `self.SetUpgrade`
  (bind _returnvalue (`self.K2_GetActorLocation` (`ActorComponent.GetOwner` (`self.StaticMeshComponent`))))
  ;[1 1 1] Tilføjer et 0.1 til ArmorUpgLevel ( Svarer til 1 level )
  (`|ExecutionSequence`
    (:`then_0`
      (`/Engine/EditorBlueprintResources/StandardMacros.DoOnce` false
        (:`Completed`
          (set `self.Price` 300.0))))
    (:`then_1`
      (bind _outactors (`GameplayStatics.GetAllActorsOfClass` "/Game/FirstPersonCPP/Blueprints/FirstPersonCharacter.FirstPersonCharacter_C"))
      (bind _output (`|GetArrayItem` _outactors))
      (if (> (`CharacterMovementComponent.MaxWalkSpeed` (`self.GetComponentByClass` _output "/Script/Engine.CharacterMovementComponent")) 1126.0)
        (`self.PlayBuzzer` (`self.K2_GetActorLocation` (`ActorComponent.GetOwner` (`self.StaticMeshComponent`))))
        (else
          (`/Game/FirstPersonCPP/Blueprints/FirstPersonCharacter.Pay` _output (`self.Price`))
          (if (`/Game/FirstPersonCPP/Blueprints/FirstPersonCharacter.CanAfford` _output)
            (`|ExecutionSequence`
              (:`then_0`
                (bind _outactors_2 (`GameplayStatics.GetAllActorsOfClass` "/Game/FirstPersonCPP/Blueprints/FirstPersonCharacter.FirstPersonCharacter_C"))
                (bind _output_2 (`|GetArrayItem` _outactors_2))
                (bind _output_get (set `/Game/FirstPersonCPP/Blueprints/FirstPersonCharacter.SpeedUpgLevel` (+ (`/Game/FirstPersonCPP/Blueprints/FirstPersonCharacter.SpeedUpgLevel` _output_2) 0.1) _output_2))
                (`|ExecutionSequence`
                  (:`then_0`
                    (bind _returnvalue_2 (* (- _output_get 1.0) 10.0))
                    (bind _returnvalue_3 (`KismetMathLibrary.Round` _returnvalue_2))
                    ;[1 1 1] Skriver max i stedet for tal, hvis man er nået max lvl ( 12 )
                    (if (>= _returnvalue_3 38)
                      (set `self.TmpString` "Max")
                      (`|ExecutionSequence`
                        (:`then_0`
                          (`GameplayStatics.PlaySoundAtLocation` "/Game/OurContent/Souund/Maxed_an_Upgrade.Maxed_an_Upgrade" _returnvalue (struct) 1.0 1.0 0.0 "/Game/OurContent/Souund/Attenuations/Button_atten.Button_atten"))
                        (:`then_1`
                          (bind _returnvalue_4 (* _returnvalue_2 300.0))
                          (set `self.Price` _returnvalue_4 :!label _label)))
                      (else
                        (set `self.TmpString` (`KismetStringLibrary.Conv_IntToString` _returnvalue_3))
                        (`|ExecutionSequence`
                          (:`then_0`
                            (goto _label))
                          (:`then_1`
                            (`GameplayStatics.PlaySoundAtLocation` "/Game/OurContent/Souund/Thuum.Thuum" _returnvalue (struct) 1.0 1.0 0.0 "/Game/OurContent/Souund/Attenuations/Button_atten.Button_atten"))))))
                  (:`then_1`
                    (bind _returnvalue_5 (`KismetMathLibrary.Conv_IntToDouble` (`KismetMathLibrary.Round` (* (`/Game/FirstPersonCPP/Blueprints/FirstPersonCharacter.Speed` _output_2) 1.025))))
                    ;[1 1 1] Applies new speed upgrades
                    (bind _output_get_2 (set `/Game/FirstPersonCPP/Blueprints/FirstPersonCharacter.Speed` _returnvalue_5 _output_2))
                    (set `CharacterMovementComponent.MaxWalkSpeed` _returnvalue_5 (`self.GetComponentByClass` _output_2 "/Script/Engine.CharacterMovementComponent")))
                  (:`then_2`
                    ;[1 1 1] Sætter teksten på Text Render
                    (set `self.TextString` (`KismetStringLibrary.Concat_StrStr` "        Speed \nPrice: " (`KismetStringLibrary.Conv_IntToString` (`KismetMathLibrary.Round` _returnvalue_4)) "$ \nCurrent level: " (`KismetStringLibrary.Conv_IntToString` (`KismetMathLibrary.Round` (- _returnvalue_2 1.0))) " \nNext level: " (`self.TmpString`) " \nCurrent bonus: \n" (`KismetStringLibrary.Conv_IntToString` (`KismetMathLibrary.Round` (* (- (/ _output_get_2 450.0) 1.0) 100.0))) "%"))
                    (`|ExecutionSequence`
                      (:`then_0`
                        ;[1 1 1] Finder TextRenderComponent, som har et navn der indeholder TrapRes og sætter den lig med TextRenderComponent variablen
                        (`/Engine/EditorBlueprintResources/StandardMacros.DoOnce` false
                          (:`Completed`
                            (bind _outactors_3 (`GameplayStatics.GetAllActorsOfClass` "/Script/Engine.TextRenderActor"))
                            (for _array_element _outactors_3
                              (if (`KismetStringLibrary.Contains` (`KismetSystemLibrary.GetObjectName` _array_element) "Speed")
                                (set `self.TextRenderComponent` (`TextRenderActor.TextRender` _array_element))
                                (`KismetSystemLibrary.PrintString` "Found TextRender"))))))
                      (:`then_1`
                        (`TextRenderComponent.K2_SetText` (`self.TextRenderComponent`) (`KismetTextLibrary.Conv_StringToText` (`self.TextString`))))))))
              (:`then_1`
                (set `self.PlayerUpgString` (`self.TmpString`))))))))))

(fn `UserConstructionScript`
  (`parent.UserConstructionScript`))