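; Upgrade button that sells percent-damage levels to the FirstPersonCharacter through the SetUpgrade event.
; It charges the player via Pay and, if affordable, raises the upgrade level and damage bonus, then plays a sound.
; The price starts fixed, then scales linearly with level.
; A TextRenderActor, found once by name, displays the price, levels and current bonus.
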(event `self.SetUpgrade`
  ;[1 1 1] Tilføjer et 0.1 til ArmorUpgLevel ( Svarer til 1 level )
  (`|ExecutionSequence`
    (:`then_0`
      (`/Engine/EditorBlueprintResources/StandardMacros.DoOnce` false
        (:`Completed`
          (set `self.Price` 200.0))))
    (:`then_1`
      (bind _outactors (`GameplayStatics.GetAllActorsOfClass` "/Game/FirstPersonCPP/Blueprints/FirstPersonCharacter.FirstPersonCharacter_C"))
      (bind _output (`|GetArrayItem` _outactors))
      (`/Game/FirstPersonCPP/Blueprints/FirstPersonCharacter.Pay` _output (`self.Price`))
      (if (`/Game/FirstPersonCPP/Blueprints/FirstPersonCharacter.CanAfford` _output)
        (`|ExecutionSequence`
          (:`then_0`
            (bind _outactors_2 (`GameplayStatics.GetAllActorsOfClass` "/Game/FirstPersonCPP/Blueprints/FirstPersonCharacter.FirstPersonCharacter_C"))
            (bind _output_2 (`|GetArrayItem` _outactors_2))
            (bind _output_get (set `/Game/FirstPersonCPP/Blueprints/FirstPersonCharacter.DmgPercentUpgLevel` (+ (`/Game/FirstPersonCPP/Blueprints/FirstPersonCharacter.DmgPercentUpgLevel` _output_2) 0.1) _output_2))
            (`|ExecutionSequence`
              (:`then_0`
                (bind _returnvalue (* (- _output_get 1.0) 10.0))
                ;[1 1 1] Sætter tallet på prisen
                (set `self.TmpString` (`KismetStringLibrary.Conv_IntToString` (`KismetMathLibrary.Round` _returnvalue)))
                (`|ExecutionSequence`
                  (:`then_0`
                    (`GameplayStatics.PlaySoundAtLocation` "/Game/OurContent/Souund/Thuum.Thuum" (`self.K2_GetActorLocation` (`ActorComponent.GetOwner` (`self.StaticMeshComponent`))) (struct) 1.0 1.0 0.0 "/Game/OurContent/Souund/Attenuations/Button_atten.Button_atten"))
                  (:`then_1`
                    (bind _returnvalue_2 (* _returnvalue 150.0))
                    (set `self.Price` _returnvalue_2))))
              (:`then_1`
                ;[1 1 1] Applies new armor upgrades
                (bind _output_get_2 (set `/Game/FirstPersonCPP/Blueprints/FirstPersonCharacter.DmgPercent` (`KismetMathLibrary.Conv_IntToDouble` (`KismetMathLibrary.Round` (+ (`/Game/FirstPersonCPP/Blueprints/FirstPersonCharacter.DmgPercent` _output_2) 20.0))) _output_2)))
              (:`then_2`
                ;[1 1 1] Sætter teksten på Text Render
                (set `self.TextString` (`KismetStringLibrary.Concat_StrStr` "Percent Damage \nPrice: " (`KismetStringLibrary.Conv_IntToString` (`KismetMathLibrary.Round` _returnvalue_2)) "$ \nCurrent level: " (`KismetStringLibrary.Conv_IntToString` (`KismetMathLibrary.Round` (- _returnvalue 1.0))) " \nNext level: " (`self.TmpString`) " \nCurrent Bonus: \n" (`KismetStringLibrary.Conv_IntToString` (`KismetMathLibrary.Round` _output_get_2)) "%"))
                (`|ExecutionSequence`
                  (:`then_0`
                    ;[1 1 1] Finder TextRenderComponent, som har et navn der indeholder PercentDamage og sætter den lig med TextRenderComponent variablen
                    (`/Engine/EditorBlueprintResources/StandardMacros.DoOnce` false
                      (:`Completed`
                        (bind _outactors_3 (`GameplayStatics.GetAllActorsOfClass` "/Script/Engine.TextRenderActor"))
                        (for _array_element _outactors_3
                          (if (`KismetStringLibrary.Contains` (`KismetSystemLibrary.GetObjectName` _array_element) "DmgPercent")
                            (set `self.TextRenderComponent` (`TextRenderActor.TextRender` _array_element))
                            (`KismetSystemLibrary.PrintString` "Found TextRender"))))))
                  (:`then_1`
                    (`TextRenderComponent.K2_SetText` (`self.TextRenderComponent`) (`KismetTextLibrary.Conv_StringToText` (`self.TextString`))))))))
          (:`then_1`
            (set `self.PlayerUpgString` (`self.TmpString`))))))))

(fn `UserConstructionScript`
  (`parent.UserConstructionScript`))